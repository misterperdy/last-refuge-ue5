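; BP_Zombie is an enemy that patrols a spline path, chases the player on sight and deals damage on hitbox overlap.
; Tick moves it directly along the looping spline, snapped to the navmesh with a height offset, unless chasing or returning.
; Pawn sensing starts an AI MoveTo at double speed.
; A retriggerable delay ends the chase three seconds after the last sighting, then walks it back to its saved spline point.
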(event OnSeePawn(PawnSensing)
  (params (Pawn :type Pawn%20Object%20Reference))
  (bind _self self)
  (bind _patrolspeed (Variables|Default|GetPatrolSpeed))
  (bind _asbp_player_character (Utilities|Casting|CastToBP_playerCharacter Pawn))
  (Variables|Default|SetisChasing true)
  (Variables|/Script/Engine.CharacterMovementComponent|SetMaxWalkSpeed (Variables|Character|GetCharacterMovement) (* _patrolspeed 2.0))
  (AI|AIMoveTo _self "0, 0, 0" _asbp_player_character 5.0 false
    (:then
      (Utilities|FlowControl|RetriggerableDelay 3.0)
      (Variables|Default|SetisChasing false)
      (Variables|Default|SetisReturning true)
      (Variables|/Script/Engine.CharacterMovementComponent|SetMaxWalkSpeed (Variables|Character|GetCharacterMovement) _patrolspeed)
      (AI|AIMoveTo _self (.ProjectedLocation (AI|Navigation|ProjectPointtoNavigation (Spline|GetLocationatDistanceAlongSpline (Variables|/Game/Project/Blueprints/BP_PatrolPath.BP_PatrolPath_C|GetSpline (Variables|Default|GetPatrolPath)) (Variables|Default|GetDistanceAlongSpline) "World") 0 0 "100.000000,100.000000,50000.000000")) 0 5.0 false
        (:OnSuccess
          (Variables|Default|SetisReturning false))))))

(event OnComponentBeginOverlap(DamageBox)
  (params (OverlappedComponent :type Primitive%20Component%20Object%20Reference) (OtherActor :type Actor%20Object%20Reference) (OtherComp :type Primitive%20Component%20Object%20Reference) (OtherBodyIndex :type Integer) (bFromSweep :type Boolean) (SweepResult :type Hit%20Result%20Structure%20%28by%20ref%29))
  (bind _asbp_player_character (Utilities|Casting|CastToBP_playerCharacter OtherActor))
  (Game|Damage|ApplyDamage _asbp_player_character 1e+01 0 self))

(event EventBeginPlay)

(event Collision|EventActorBeginOverlap
  (params (OtherActor :type Actor%20Object%20Reference)))

(event EventTick
  (params (DeltaSeconds :type Float%20%28single-precision%29))
  (bind _patrolpath (Variables|Default|GetPatrolPath))
  (bind _spline (Variables|/Game/Project/Blueprints/BP_PatrolPath.BP_PatrolPath_C|GetSpline _patrolpath))
  (if (not (or (Variables|Default|GetisChasing) (Variables|Default|GetisReturning)))
    (Utilities|IsValid _patrolpath
      (:Is%20Valid
        (Variables|Default|SetDistanceAlongSpline (Math|Float|%(Float) (+ (* DeltaSeconds (Variables|Default|GetPatrolSpeed)) (Variables|Default|GetDistanceAlongSpline)) (Spline|GetSplineLength _spline)))
        (Transformation|SetActorLocationAndRotation (Math|Vector|MakeVector (.x (.ProjectedLocation (AI|Navigation|ProjectPointtoNavigation (Spline|GetLocationatDistanceAlongSpline _spline (Math|Float|%(Float) (+ (* DeltaSeconds (Variables|Default|GetPatrolSpeed)) (Variables|Default|GetDistanceAlongSpline)) (Spline|GetSplineLength _spline)) "World") 0 0 "0, 0, 0"))) (.y (.ProjectedLocation (AI|Navigation|ProjectPointtoNavigation (Spline|GetLocationatDistanceAlongSpline _spline (Math|Float|%(Float) (+ (* DeltaSeconds (Variables|Default|GetPatrolSpeed)) (Variables|Default|GetDistanceAlongSpline)) (Spline|GetSplineLength _spline)) "World") 0 0 "0, 0, 0"))) (+ (.z (.ProjectedLocation (AI|Navigation|ProjectPointtoNavigation (Spline|GetLocationatDistanceAlongSpline _spline (Math|Float|%(Float) (+ (* DeltaSeconds (Variables|Default|GetPatrolSpeed)) (Variables|Default|GetDistanceAlongSpline)) (Spline|GetSplineLength _spline)) "World") 0 0 "0, 0, 0"))) 75.0)) (Spline|GetRotationatDistanceAlongSpline _spline (Math|Float|%(Float) (+ (* DeltaSeconds (Variables|Default|GetPatrolSpeed)) (Variables|Default|GetDistanceAlongSpline)) (Spline|GetSplineLength _spline)) "World"))))))

(fn ConstructionScript)