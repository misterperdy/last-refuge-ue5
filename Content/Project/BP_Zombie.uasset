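; BP_Zombie is a zombie actor that patrols along the spline of its assigned PatrolPath.
; Each Tick, while the path is valid, it advances a distance along the spline by PatrolSpeed and delta time, wrapping by modulo of spline length to loop.
; It sets its world location and rotation directly from the spline, with no AI or navigation logic in the graph.
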(event EventBeginPlay)

(event Collision|EventActorBeginOverlap
  (params (OtherActor :type Actor%20Object%20Reference)))

(event EventTick
  (params (DeltaSeconds :type Float%20%28single-precision%29))
  (bind _patrolpath (Variables|Default|GetPatrolPath))
  (bind _spline (Variables|/Game/Project/BP_PatrolPath.BP_PatrolPath_C|GetSpline _patrolpath))
  (Utilities|IsValid _patrolpath
    (:Is%20Valid
      (Variables|Default|SetDistanceAlongSpline (Math|Float|%(Float) (+ (* DeltaSeconds (Variables|Default|GetPatrolSpeed)) (Variables|Default|GetDistanceAlongSpline)) (Spline|GetSplineLength _spline)))
      (Transformation|SetActorLocationAndRotation (Spline|GetLocationatDistanceAlongSpline _spline (Math|Float|%(Float) (+ (* DeltaSeconds (Variables|Default|GetPatrolSpeed)) (Variables|Default|GetDistanceAlongSpline)) (Spline|GetSplineLength _spline)) "World") (Spline|GetRotationatDistanceAlongSpline _spline (Math|Float|%(Float) (+ (* DeltaSeconds (Variables|Default|GetPatrolSpeed)) (Variables|Default|GetDistanceAlongSpline)) (Spline|GetSplineLength _spline)) "World")))))

(fn ConstructionScript)